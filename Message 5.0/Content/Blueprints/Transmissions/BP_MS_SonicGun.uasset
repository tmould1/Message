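; BP_MS_SonicGun is a gun actor that fires BP_MS_Bullet projectiles in a 2D side-scroller.
; Tick accumulates time since the last shot, and FireGun only fires once that exceeds the fire sound's length.
; Bullets spawn at BulletSpawnPoint but take the player's Y to stay on their plane, then rotate 90 degrees.
; Each shot plays a fading gunshot and triggers the player character's gunshot reaction.
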(event `self.ReceiveBeginPlay`)

(event `self.ReceiveTick`
  (params (DeltaSeconds :type "Float (single-precision)"))
  (set `self.secondsSinceLastFired` (+ (`self.secondsSinceLastFired`) DeltaSeconds)))

(fn `FireGun`
  (bind _gunshot (`self.GunShot`))
  (bind _returnvalue (`SceneComponent.K2_GetComponentToWorld` (`self.BulletSpawnPoint`)))
  (bind (_returnvalue_x _returnvalue_y) (`KismetMathLibrary.BreakVector` (`self.K2_GetActorLocation` (`GameplayStatics.GetPlayerPawn` 0))))
  (bind (_as2dside_scroller_character _bsuccess) (cast `/Game/2DSideScrollerBP/Blueprints/2DSideScrollerCharacter` (`GameplayStatics.GetPlayerPawn` 0) :!pure true))
  (if (> (`self.secondsSinceLastFired`) (`self.lengthOfFireSound`))
    (set `self.secondsSinceLastFired` 0.0)
    (bind _returnvalue_2 (`|SpawnActorFromClass` "/Game/Blueprints/Transmissions/BP_MS_Bullet.BP_MS_Bullet_C" (`KismetMathLibrary.MakeTransform` (`KismetMathLibrary.MakeVector` (.x (.location _returnvalue)) _returnvalue_y (.z (.location _returnvalue))) (.rotation _returnvalue)) "AlwaysSpawn" "OverrideRootScale" null null))
    (`|ExecutionSequence`
      (:`then_0`
        (`AudioComponent.Play` _gunshot 0.0)
        (`AudioComponent.FadeOut` _gunshot 1.0 0.0 "Linear")
        (`self.K2_AddActorLocalRotation` _returnvalue_2 (struct :`Pitch` 90.0) false false))
      (:`then_1`
        (if _bsuccess
          (`/Game/2DSideScrollerBP/Blueprints/2DSideScrollerCharacter.PlayGunShotReaction` _as2dside_scroller_character false))))))

(fn `UserConstructionScript`)