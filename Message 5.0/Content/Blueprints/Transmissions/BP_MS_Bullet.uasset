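; Bullet actor that bounces off BP_MS_Reflector actors and destroys itself on hitting anything else, with a short lifespan set at BeginPlay.
; On a reflector hit, it turns a quarter circle in local space and teleports to the hit location.
; It then casts BulletProjectile to AudioHelper to resolve a soft-referenced SoundCue and play it there, skipping the sound if a cast fails.
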(event `self.ReceiveBeginPlay`
  (`self.SetLifeSpan` 5.0))

(event `self.ReceiveHit`
  (params (MyComp :type "PrimitiveComponent Object Reference") (Other :type "Actor Object Reference") (OtherComp :type "PrimitiveComponent Object Reference") (bSelfMoved :type Boolean) (HitLocation :type "Vector Structure") (HitNormal :type "Vector Structure") (NormalImpulse :type "Vector Structure") (Hit :type "HitResult Structure (by ref)"))
  (if (`.bSuccess` (cast `/Game/Blueprints/Transmissions/Reactors/BP_MS_Reflector` Other :!pure true))
    (`self.K2_AddActorLocalRotation` (struct :`Pitch` 90.0))
    (`self.K2_SetActorLocation` HitLocation)
    (bind _asaudio_helper (cast `/Game/Audio/AudioHelper` (`self.BulletProjectile`)))
    (bind _outsoundcue (`/Game/Audio/AudioHelper.GetSound` _asaudio_helper (`self.In Sound Cue Soft Ref`)))
    (bind _requestedsound (`/Game/Audio/AudioHelper.RespondToAsyncLoadFinished` _asaudio_helper _outsoundcue))
    (bind _assound_cue (cast `SoundCue` _requestedsound))
    (`GameplayStatics.PlaySoundAtLocation` _assound_cue HitLocation (struct) 1.0 1.0 0.0 null null null)
    (else
      (`self.K2_DestroyActor`))))

(fn `UserConstructionScript`)