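; BP_MS_TurnItUpToEleven is a transmission reactor that moves the game to another level when it reacts.
; DoReact runs once, waits a few seconds, then reads ShouldLoadOutro from MS_GameInstance.
; It opens OutroScene if that flag is set, and MainMenu if the flag is unset or the game instance cast fails.
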(event `self.DoReact`
  (params (hitResult :type "HitResult Structure"))
  (bind (_asms_game_instance _bsuccess) (cast `/Game/MS_GameInstance` (`GameplayStatics.GetGameInstance`) :!pure true))
  (`/Engine/EditorBlueprintResources/StandardMacros.DoOnce` false
    (:`Completed`
      (`|ExecutionSequence`
        (:`then_1`
          (`KismetSystemLibrary.Delay` 3.0)
          (if _bsuccess
            (if (`/Game/MS_GameInstance.bShouldLoadOutro` _asms_game_instance)
              (`GameplayStatics.OpenLevel` "OutroScene" false)
              (else
                (`GameplayStatics.OpenLevel` "MainMenu" false :!label _label)))
            (else
              (goto _label))))))))

(fn `UserConstructionScript`
  (`parent.UserConstructionScript`))