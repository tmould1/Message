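; Base 2D flipbook enemy character with a simple state machine and hit reactions.
; Tick swaps running and idle flipbooks by velocity, flips control yaw to face horizontal movement, then dispatches AiState to Idle, Pathing, Chasing, Attacking or Pose functions, all empty stubs here.
; Capsule overlap with Debris triggers death through a short lifespan and calls a sound, while a BP_MS_Bullet overlap switches the state to Posing.
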(event `self.ReceiveBeginPlay`)

(event `UpdateAnimation`
  ;[1 1 1] Handle Animation
  (`PaperFlipbookComponent.SetFlipbook` (`self.Sprite`) (select `bool` (> (`KismetMathLibrary.VSize` (`self.GetVelocity`)) 0.0) :`false` "/Game/2DSideScroller/Sprites/IdleAnimation.IdleAnimation" :`true` "/Game/2DSideScroller/Sprites/RunningAnimation.RunningAnimation" :!type "PaperFlipbook Object Reference")))

(event `self.ReceiveTick`
  (params (DeltaSeconds :type "Float (single-precision)"))
  (`|ExecutionSequence`
    (:`then_0`
      ;[1 1 1] Animation Update
      (`self.UpdateAnimation`)
      (`/Engine/EditorBlueprintResources/StandardMacros.CompareFloat` (.x (`MovementComponent.Velocity` (`self.GetMovementComponent`)))
        (:`>`
          (`Controller.SetControlRotation` (`self.GetController`) (`KismetMathLibrary.MakeRotator` 0.0) :!label _label))
        (:`==`
          (if (`self.bIsMovingRight`)
            (goto _label)
            (else
              (`Controller.SetControlRotation` (`self.GetController`) (`KismetMathLibrary.MakeRotator` 0.0 0.0 180.0) :!label _label_2))))
        (:`<`
          (goto _label_2))))
    (:`then_1`
      ;[1 1 1] AI update
      (switch `/Game/Blueprints/E_EnemyState` (`self.aiState`)
        (:`NewEnumerator0`
          (`self.DoIdle`))
        (:`NewEnumerator1`
          (`self.DoPathing`))
        (:`NewEnumerator2`
          (`self.DoChasing` null))
        (:`NewEnumerator3`
          (`self.DoAttacking`))
        (:`NewEnumerator4`
          (`self.DoPose`))))))

(event `self.CapsuleComponent.OnComponentBeginOverlap`
  (params (OverlappedComponent :type "PrimitiveComponent Object Reference") (OtherActor :type "Actor Object Reference") (OtherComp :type "PrimitiveComponent Object Reference") (OtherBodyIndex :type Integer) (bFromSweep :type Boolean) (SweepResult :type "HitResult Structure (by ref)"))
  ;[0.004252 0 1] Hit React
  (if (`.bSuccess` (cast `/Game/Blueprints/Debris` OtherActor :!pure true))
    (`self.DoDeath`)
    (`GameplayStatics.PlaySoundAtLocation` null (`self.K2_GetActorLocation`))
    (elif (`.bSuccess` (cast `/Game/Blueprints/Transmissions/BP_MS_Bullet` OtherActor :!pure true))
      (set `self.aiState` "NewEnumerator4"))))

(fn `DoAttacking`)

(fn `DoChasing`
  (params (chaseActor :type "Actor Object Reference")))

(fn `DoDeath`
  (`self.SetLifeSpan` 0.1))

(fn `DoIdle`)

(fn `DoPathing`)

(fn `DoPose`)

(fn `UserConstructionScript`)