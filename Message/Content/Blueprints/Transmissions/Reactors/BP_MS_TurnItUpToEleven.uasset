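; A transmission reactor Blueprint that puts on a disco light show when triggered, then sends the game back to the main menu.
; DoReact fires only once, unhiding the DiscoLight and Cube components.
; The CycleColors timeline drives the light's color and restarts itself on finish, looping while a short delay runs before the MainMenu level opens.
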(event `self.DoReact`
  (params (hitResult :type "HitResult Structure"))
  (`/Engine/EditorBlueprintResources/StandardMacros.DoOnce` false
    (:`Completed`
      (`SceneComponent.SetHiddenInGame` (`self.Disco Light`) false false)
      (`SceneComponent.SetHiddenInGame` (`self.Cube`) false false)
      (`|ExecutionSequence`
        (:`then_0`
          (bind (_direction _colors) (`Timeline|CycleColors` :!label _label)
            (:`Update`
              (`LightComponent.SetLightColor` (`self.Disco Light`) _colors false))
            (:`Finished`
              (goto _label :!via `PlayFromStart`))))
        (:`then_1`
          (`KismetSystemLibrary.Delay` 5.0)
          (`GameplayStatics.OpenLevel` "MainMenu" false))))))

(fn `UserConstructionScript`
  (`parent.UserConstructionScript`))