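; BP_MS_TranslatingObject is an actor that slides between two placed points when its DoReact event fires.
; BeginPlay caches the world locations of StartingPosition and EndingPosition, and the Translate timeline's Alpha interpolates the actor between them without sweep.
; DoReact ignores calls mid-move and plays or reverses the timeline by IsInStartingPosition.
; That flag resets on finish to Alpha < 0, so it reads false at both zero and positive Alpha.
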(event `self.ReceiveBeginPlay`
  (`parent.ReceiveBeginPlay`)
  (set `self.start` (`SceneComponent.K2_GetComponentLocation` (`self.StartingPosition`)))
  (set `self.end` (`SceneComponent.K2_GetComponentLocation` (`self.EndingPosition`))))

(event `self.DoReact`
  (if (`self.timelineHasFinished`)
    (set `self.timelineHasFinished` false)
    (if (`self.isInStartingPosition`)
      (bind (_direction _alpha) (`Timeline|Translate` :!label _label)
        (:`Update`
          (`self.K2_SetActorLocation` (+ (`self.start`) (* (- (`self.end`) (`self.start`)) _alpha))))
        (:`Finished`
          (set `self.timelineHasFinished` true)
          (set `self.isInStartingPosition` (< _alpha 0.0))))
      (else
        (goto _label :!via `ReverseFromEnd`)))))

(fn `UserConstructionScript`
  (`parent.UserConstructionScript`))