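; A movable crate that the player can pick up and release through its DoReact event.
; Each DoReact call toggles an IsAttached flag, either attaching the crate actor to player 0's pawn or detaching it.
; Both operations keep world transform, so the crate follows the pawn from its current offset and stays where it is released.
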(event `self.DoReact`
  (params (gunTransform :type "Transform Structure"))
  (if (`self.isAttached`)
    (`self.K2_DetachFromActor` "KeepWorld" "KeepWorld" "KeepWorld")
    (set `self.isAttached` false)
    (else
      (`self.K2_AttachToActor` (`GameplayStatics.GetPlayerPawn` 0) "None" "KeepWorld" "KeepWorld" "KeepWorld")
      (set `self.isAttached` true))))

(fn `UserConstructionScript`)