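; Trapdoor Blueprint with two Paper2D sprites that toggles between its starting and swung positions each time DoReact is triggered.
; The Rotate timeline pitches two arrow components up to 90 degrees in opposite directions, playing forward or in reverse with a separate sound for each.
; Sprite collision is off while the timeline updates and restored when it finishes.
; A finished flag ignores triggers mid-swing, and the final timeline value decides the next direction.
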(event `self.DoReact`
  (params (gunTransform :type "Transform Structure"))
  (if (`self.timelineHasFinished`)
    (set `self.timelineHasFinished` false)
    (if (`self.isInStartingPosition`)
      (`TimelineComponent.SetPlayRate` (`self.Rotate`) 4.0)
      (`GameplayStatics.PlaySound2D` "/Game/Audio/RAW/Trap_Door.Trap_Door")
      (bind (_direction _gamma) (`Timeline|Rotate` :!label _label)
        (:`Update`
          (bind _returnvalue (* (`KismetMathLibrary.MakeRotator` 0.0 90.0) _gamma))
          (`SceneComponent.K2_SetRelativeRotation` (`self.Arrow1`) (* _returnvalue -1.0) false false)
          (`SceneComponent.K2_SetRelativeRotation` (`self.Arrow`) _returnvalue false false)
          (`PrimitiveComponent.SetCollisionEnabled` (`self.PaperSprite`) "NoCollision")
          (`PrimitiveComponent.SetCollisionEnabled` (`self.PaperSprite1`) "NoCollision"))
        (:`Finished`
          (set `self.TimelineHasFinished` true)
          (set `self.IsInStartingPosition` (< _gamma 0.5))
          (`PrimitiveComponent.SetCollisionEnabled` (`self.PaperSprite`) "QueryAndPhysics")
          (`PrimitiveComponent.SetCollisionEnabled` (`self.PaperSprite1`) "QueryAndPhysics")))
      (else
        (`GameplayStatics.PlaySound2D` "/Game/Audio/RAW/Trap_door_reset.Trap_door_reset")
        (goto _label :!via `Reverse`)))))

(fn `UserConstructionScript`
  (`parent.UserConstructionScript`))