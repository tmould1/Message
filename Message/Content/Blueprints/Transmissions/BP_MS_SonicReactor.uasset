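; BP_MS_SonicReactor is an actor that reacts to bullets, with an empty DoReact hook as the response.
; When its InteractorField is hit by a BP_MS_Bullet, it passes the hit to DoReact.
; Event_GunFired line-traces from the gun to the actor and, if unblocked, delays by distance over speed to match travel time.
; Nothing runs after that delay, so the gunfire path triggers no reaction.
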(event `self.ReceiveBeginPlay`)

(event `self.InteractorField.OnComponentHit`
  (params (HitComponent :type "PrimitiveComponent Object Reference") (OtherActor :type "Actor Object Reference") (OtherComp :type "PrimitiveComponent Object Reference") (NormalImpulse :type "Vector Structure") (Hit :type "HitResult Structure (by ref)"))
  (if (`.bSuccess` (cast `/Game/Blueprints/Transmissions/BP_MS_Bullet` OtherActor :!pure true))
    (`self.DoReact` Hit)))

(event `Event_GunFired`
  (params (origin :type "Transform Structure") (speed :type "Float (double-precision)"))
  (bind _returnvalue (`self.K2_GetActorLocation`))
  (bind _output_get (set `self.gunTransform` origin))
  (bind (_outhit _returnvalue_2) (`KismetSystemLibrary.LineTraceSingle` (.location _output_get) _returnvalue "TraceTypeQuery3" true))
  ;[1 1 1] if hit is true, shot was blocked.
  (if (not _returnvalue_2)
    (`KismetSystemLibrary.Delay` (/ (`KismetMathLibrary.VSize` (- (.location _output_get) _returnvalue)) speed))))

(fn `DoReact`
  (params (hitResult :type "HitResult Structure")))

(fn `UserConstructionScript`)