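; BP_MS_PartyAnimal is an enemy Blueprint with enum-based AI state events that can kill the side-scroller player.
; A capsule hit on the player changes the state, and DoAttacking calls the player's DoDeath before resetting it.
; Idle only waits and checks state, while pathing, chasing and sight events are empty.
; Random-roam and chase AIMoveTo logic remains in the graph but is disconnected and never runs.
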(event `self.DoIdle`
  ;[1 1 1] State Behavior
  (`KismetSystemLibrary.Delay` 3.0)
  (if (`|EnumEquality` (`self.aiState`) "NewEnumerator0")
    _))

(event `self.DoPathing`
  ;[1 1 1] State Behavior
)

(event `self.PawnSensing.OnSeePawn`
  (params (Pawn :type "Pawn Object Reference")))

(event `self.DoChasing`
  (params (chaseActor :type "Actor Object Reference"))
  ;[1 1 1] State Behavior
)

(event `self.DoAttacking`
  ;[1 1 1] State Behavior
  (`/Game/2DSideScrollerBP/Blueprints/2DSideScrollerCharacter.DoDeath` (cast `/Game/2DSideScrollerBP/Blueprints/2DSideScrollerCharacter` (`GameplayStatics.GetPlayerPawn` 0) :!pure true))
  (set `self.aiState` "NewEnumerator0"))

(event `self.CapsuleComponent.OnComponentHit`
  (params (HitComponent :type "PrimitiveComponent Object Reference") (OtherActor :type "Actor Object Reference") (OtherComp :type "PrimitiveComponent Object Reference") (NormalImpulse :type "Vector Structure") (Hit :type "HitResult Structure (by ref)"))
  (if (`.bSuccess` (cast `/Game/2DSideScrollerBP/Blueprints/2DSideScrollerCharacter` OtherActor :!pure true))
    (set `self.aiState` "NewEnumerator3")))

(fn `UserConstructionScript`
  (`parent.UserConstructionScript`))