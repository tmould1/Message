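; BP_MS_Beater is a side-scroller enemy that patrols, chases the player on sight and kills them.
; It supplies behavior events for AiState values, with no dispatch in this graph.
; Random idle pauses lead into AIMoveTo patrols that alternate direction along X, while PawnSensing switches it to chasing.
; When the chase move finishes, the attack calls the player's DoDeath without a range check and returns to idle.
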(event `self.DoIdle`
  ;[1 1 1] State Behavior
  (`KismetSystemLibrary.Delay` (* (`KismetMathLibrary.RandomFloat`) 3.0))
  (if (`|EnumEquality` (`self.aiState`) "NewEnumerator0")
    (set `self.aiState` "NewEnumerator1")))

(event `self.DoPathing`
  (bind (_returnvalue_x _returnvalue_y _returnvalue_z) (`KismetMathLibrary.BreakVector` (`self.K2_GetActorLocation`)))
  (bind _navpathawaydistance (`self.navPathAwayDistance`))
  ;[1 1 1] State Behavior
  (if (`self.bPathingFinished`)
    (set `self.bPathingFinished` false)
    (bind _result (`/Engine/EditorBlueprintResources/StandardMacros.IncrementInt` (`self.numTimesPathed`))
      (:`  `
        (if (== (mod _result 2) 0)
          (`|AIMoveTo` self (`KismetMathLibrary.MakeVector` (+ _returnvalue_x _navpathawaydistance) _returnvalue_y _returnvalue_z) null 5.0
            (:`OnSuccess`
              _)
            (:`OnFail`
              _))
          (else
            (`|AIMoveTo` self (`KismetMathLibrary.MakeVector` (- _returnvalue_x _navpathawaydistance) _returnvalue_y _returnvalue_z) null 5.0
              (:`OnSuccess`
                _)
              (:`OnFail`
                _))))
        (set `self.aiState` "NewEnumerator0")
        (set `self.bPathingFinished` true)))))

(event `self.PawnSensing.OnSeePawn`
  (params (Pawn :type "Pawn Object Reference"))
  (if (`|EnumInequality` (`self.aiState`) "NewEnumerator2")
    (set `self.aiState` "NewEnumerator2")))

(event `self.DoChasing`
  (params (chaseActor :type "Actor Object Reference"))
  ;[1 1 1] State Behavior
  (`AITask_MoveTo.AIMoveTo` (`AIBlueprintHelperLibrary.GetAIController` (`self.GetController`)) (0.0 0.0 0.0) (`GameplayStatics.GetPlayerPawn` 0) 2.0 "Enable"
    (:`OnMoveFinished`
      (set `self.aiState` "NewEnumerator3"))))

(event `self.DoAttacking`
  ;[1 1 1] State Behavior
  (`/Game/2DSideScrollerBP/Blueprints/2DSideScrollerCharacter.DoDeath` (cast `/Game/2DSideScrollerBP/Blueprints/2DSideScrollerCharacter` (`GameplayStatics.GetPlayerPawn` 0) :!pure true))
  (set `self.aiState` "NewEnumerator0"))

(event `self.DoPose`
  ;[1 1 1] State Behavior
)

(fn `UserConstructionScript`
  (`parent.UserConstructionScript`))